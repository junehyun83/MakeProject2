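; Parkour component that detects obstacles ahead of its owning character and vaults over them.
; TriggerParkour runs layered sphere and line traces to find the wall face, top edges and landing spot, then measures wall height.
; Grounded, moving characters get a one-hand vault, two-hand vault or front flip by height; mantle and climb only print.
; Vaults play montages in flying mode without capsule collision, with motion-warp targets for two-hand and flip.
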(event `self.ReceiveTick`
  (params (DeltaSeconds :type "Float (single-precision)"))
  (bind _returnvalue (`SceneComponent.K2_GetComponentLocation` (`self.PlayerMesh`)))
  ;[1 1 1] Comment
  (bind (_outhit _returnvalue_2) (`KismetSystemLibrary.SphereTraceSingle` :`Start` _returnvalue :`End` _returnvalue :`Radius` (`CapsuleComponent.CapsuleRadius` (`self.PlayerCapsule`)) :`TraceChannel` "TraceTypeQuery1" :`DrawDebugType` "ForOneFrame"))
  (set `self.IsOnLand` _returnvalue_2))

(event `TryVault`
  (params (VaultType :type "/Game/CustomContents/Enum_VaultType Enum" :default "NewEnumerator0"))
  (bind _wallrotation (`self.WallRotation`))
  (bind _wallrotation_2 (`self.WallRotation`))
  (bind _wallrotation_3 (`self.WallRotation`))
  (bind _playermesh (`self.PlayerMesh`))
  ;[1 1 1] Comment
  (set `self.CanParkour` false)
  (`PrimitiveComponent.SetCollisionEnabled` (`self.PlayerCapsule`) "NoCollision")
  (`CharacterMovementComponent.SetMovementMode` (`self.CharacterMovement`) "MOVE_Flying" 0)
  (switch `/Game/CustomContents/Enum_VaultType` VaultType
    (:`NewEnumerator0`
      (`|PlayMontage` _playermesh "/Game/CustomContents/Animation/Montage/OneHandVault_Montage.OneHandVault_Montage"
        (:`OnCompleted`
          (set `self.CanParkour` true :!label _label))
        (:`OnBlendOut`
          (`PrimitiveComponent.SetCollisionEnabled` (`self.PlayerCapsule`) "QueryAndPhysics" :!label _label_2)
          (`CharacterMovementComponent.SetMovementMode` (`self.CharacterMovement`) "MOVE_Walking" 0))))
    (:`NewEnumerator1`
      (`MotionWarpingComponent.AddOrUpdateWarpTargetFromLocationAndRotation` (`self.MotionWraping`) "VaultStart" (`/Game/CustomContents/BP_Helper.MoveVectorDownward` (`/Game/CustomContents/BP_Helper.MoveVectorForward` (`.Location` (`GameplayStatics.BreakHitResult` (`self.FirstTopHitResult`))) _wallrotation_3 62.0) 46.5) _wallrotation_3)
      (`MotionWarpingComponent.AddOrUpdateWarpTargetFromLocationAndRotation` (`self.MotionWraping`) "VaultEnd" (`.Location` (`GameplayStatics.BreakHitResult` (`self.VaultLandingHitResult`))) (`self.WallRotation`))
      (`|PlayMontage` _playermesh "/Game/CustomContents/Animation/Montage/TwoHandVault_Montage.TwoHandVault_Montage"
        (:`OnCompleted`
          (goto _label))
        (:`OnBlendOut`
          (goto _label_2))))
    (:`NewEnumerator2`
      (`MotionWarpingComponent.AddOrUpdateWarpTargetFromLocationAndRotation` (`self.MotionWraping`) "VaultStart" (`/Game/CustomContents/BP_Helper.MoveVectorBackward` (`.Location` (`GameplayStatics.BreakHitResult` (`self.FirstTopHitResult`))) _wallrotation 100.0) _wallrotation)
      (`MotionWarpingComponent.AddOrUpdateWarpTargetFromLocationAndRotation` (`self.MotionWraping`) "VaultEnd" (`/Game/CustomContents/BP_Helper.MoveVectorRight` (`.Location` (`GameplayStatics.BreakHitResult` (`self.VaultLandingHitResult`))) _wallrotation_2 5.0) _wallrotation_2)
      (`|PlayMontage` _playermesh "/Game/CustomContents/Animation/Montage/FrontFlip_Montage.FrontFlip_Montage"
        (:`OnCompleted`
          (goto _label))
        (:`OnBlendOut`
          (goto _label_2))))))

(fn `DetectWall`
  (returns (ReturnValue :type Boolean) (HitLocation :type "Vector Structure") (ReverseNormal :type "Rotator Structure"))
  (bind _returnvalue (`self.GetOwner`))
  ;[1 1 1] Player 전방의 SphereTrace 생성
  (for _index (range 8)
    (bind _returnvalue_2 (`/Game/CustomContents/BP_Helper.MoveVectorUpward` (`/Game/CustomContents/BP_Helper.MoveVectorDownward` (`Actor.K2_GetActorLocation` _returnvalue) 60.0) (* _index 20.0)))
    (bind (_outhit _returnvalue_3) (`KismetSystemLibrary.SphereTraceSingle` :`Start` (`/Game/CustomContents/BP_Helper.MoveVectorBackward` _returnvalue_2 (`Actor.K2_GetActorRotation` _returnvalue) 30.0) :`End` (+ _returnvalue_2 (* (`Actor.GetActorForwardVector` _returnvalue) 200.0)) :`Radius` 10.0 :`TraceChannel` "TraceTypeQuery1" :`DrawDebugType` "ForOneFrame"))
    (if _returnvalue_3
      (`|ExecutionSequence`
        (:`then_0`
          (break))
        (:`then_1`
          (bind (_bblockinghit _binitialoverlap _time _distance _location _impactpoint _normal) (`GameplayStatics.BreakHitResult` _outhit))
          (return _bblockinghit _location (`/Game/CustomContents/BP_Helper.ReverseNormal` _normal)))))))

(fn `Initialize`
  (bind _returnvalue (`self.GetOwner`))
  ;[1 1 1] Character Mesh
  (bind _returnvalue_2 (message `/Game/CustomContents/Interfaces/BPI_Player.GetMesh` _returnvalue))
  (set `self.PlayerMesh` _returnvalue_2)
  ;[1 1 1] Character Capsule
  (bind _returnvalue_3 (message `/Game/CustomContents/Interfaces/BPI_Player.GetPlayerCapsule` _returnvalue))
  (set `self.PlayerCapsule` _returnvalue_3)
  ;[1 1 1] Character Movement
  (bind _returnvalue_4 (message `/Game/CustomContents/Interfaces/BPI_Player.GetCharacterMovement` _returnvalue))
  (set `self.CharacterMovement` _returnvalue_4)
  ;[1 1 1] MotionWraping
  (bind _returnvalue_5 (message `/Game/CustomContents/Interfaces/BPI_Player.GetMotionWraping` _returnvalue))
  (set `self.MotionWraping` _returnvalue_5))

(fn `MeasureWall`
  (if (and (`GameplayStatics.BreakHitResult` (`self.FacedWallHitResult`)) (`GameplayStatics.BreakHitResult` (`self.FirstTopHitResult`)))
    ;[1 1 1] Wall의 높이 계산
    (set `self.WallHeight` (- (.z (`.ImpactPoint` (`GameplayStatics.BreakHitResult` (`self.FirstTopHitResult`)))) (.z (`SceneComponent.K2_GetComponentLocation` (`self.PlayerMesh`)))))
    (else
      (set `self.WallHeight` 0.0))))

(fn `ScanWall`
  (params (DetectLocation :type "Vector Structure") (ReversedNormal :type "Rotator Structure"))
  (bind _reversednormal (`local.ReversedNormal`))
  (bind (_bblockinghit _binitialoverlap _time _distance _location _impactpoint) (`GameplayStatics.BreakHitResult` (`self.LastTopHitResult`)))
  (bind (_bblockinghit_2 _binitialoverlap_2 _time_2 _distance_2 _location_2 _impactpoint_2 _normal) (`GameplayStatics.BreakHitResult` (`self.FacedWallHitResult`)))
  ;[1 1 1] Hit이 발생 시 Z축으로 2차 Scan (충돌 지점의 위 300에서 밑으로 LineTrace를 30번 수행)
  (for _index (range 30)
    (bind _returnvalue (`/Game/CustomContents/BP_Helper.MoveVectorDownward` (`/Game/CustomContents/BP_Helper.MoveVectorUpward` (`local.DetectLocation`) 300.0) (* _index 10)))
    (bind (_outhit _returnvalue_2) (`KismetSystemLibrary.LineTraceSingle` (`/Game/CustomContents/BP_Helper.MoveVectorBackward` _returnvalue _reversednormal 20.0) (`/Game/CustomContents/BP_Helper.MoveVectorForward` _returnvalue _reversednormal 80.0) "TraceTypeQuery1"))
    (if _returnvalue_2
      (set `self.FacedWallHitResult` _outhit)
      (break)))
  ;[1 1 1] Scan 이후 Hit 된 부분에서 X,Z축으로 3차 Scan (충돌 지점에서 위에서 아래로 SphereTrace를 10번 수행)
  (set `self.WallRotation` (`/Game/CustomContents/BP_Helper.ReverseNormal` _normal))
  (for _index_2 (range 10)
    (bind _returnvalue_3 (`/Game/CustomContents/BP_Helper.MoveVectorUpward` (`/Game/CustomContents/BP_Helper.MoveVectorForward` _location_2 (`self.WallRotation`) (* _index_2 20)) 10.0))
    (bind (_outhit_2 _returnvalue_4) (`KismetSystemLibrary.SphereTraceSingle` _returnvalue_3 (`/Game/CustomContents/BP_Helper.MoveVectorDownward` _returnvalue_3 10.0) 5.0 "TraceTypeQuery1"))
    ;[1 1 1] First/Last Top Hit Result의 정보
    (if (== _index_2 0)
      (if _returnvalue_4
        (bind _output_get (set `self.FirstTopHitResult` _outhit_2)) ; Hit 시 Player와 Actor의 가장 가까운 거리의 지점
        (`KismetSystemLibrary.DrawDebugSphere` (`.ImpactPoint` (`GameplayStatics.BreakHitResult` _output_get)) 5.0 12 (struct :`G` 1.0 :`A` 1.0) 10.0))
      (elif _returnvalue_4
        (set `self.LastTopHitResult` _outhit_2) ; Hit 시 Player와 Actor의 가장 먼 거리의 지점
        (else
          (`|ExecutionSequence`
            (:`then_0`
              (break))
            (:`then_1`
              ;[1 1 1] LastTopHit 부분에서 X축 +20에 SphereTrace 생성
              (bind (_outhit_3 _returnvalue_5) (`KismetSystemLibrary.SphereTraceSingle` (`/Game/CustomContents/BP_Helper.MoveVectorForward` _impactpoint (`self.WallRotation`) 20.0) _impactpoint 10.0 "TraceTypeQuery1"))
              (if _returnvalue_5
                ;[1 1 1] VaultLanding(최종 도착) 지점 생성
                (bind _output_get_2 (set `self.EndOfWallHitResult` _outhit_3))
                (bind (_bblockinghit_3 _binitialoverlap_3 _time_3 _distance_3 _location_3 _impactpoint_3) (`GameplayStatics.BreakHitResult` _output_get_2))
                ;[1 1 1] EndOfWallHitResult의 충돌 정보 시각적 위치 생성
                (`KismetSystemLibrary.DrawDebugSphere` _impactpoint_3 5.0 12 (struct :`R` 1.0 :`G` 1.0 :`A` 1.0) 10.0)
                (bind _returnvalue_6 (`/Game/CustomContents/BP_Helper.MoveVectorForward` _impactpoint_3 (`self.WallRotation`) 60.0))
                (bind (_outhit_4 _returnvalue_7) (`KismetSystemLibrary.SphereTraceSingle` _returnvalue_6 (`/Game/CustomContents/BP_Helper.MoveVectorDownward` _returnvalue_6 180.0) 10.0 "TraceTypeQuery1"))
                (if _returnvalue_7
                  (set `self.VaultLandingHitResult` _outhit_4))))))))))

(fn `TriggerParkour`
  (bind (_returnvalue _hitlocation _reversenormal) (`self.DetectWall`)) ; 매 Tick마다 실행
  (if _returnvalue
    (`self.ScanWall` _hitlocation _reversenormal) ; Detect Wall에 Detect될 시 Scan Wall 실행
    (`self.MeasureWall`) ; Hit된 Wall과 PlayerMesh를 통한 높이 측정
    (`self.TryParkour`)))

(fn `TryParkour`
  (if (`GameplayStatics.BreakHitResult` (`self.FirstTopHitResult`))
    (if (`self.IsOnLand`)
      (if (<= (`self.WallHeight`) 300.0)
        (if (<= (`self.WallHeight`) 130.0)
          (if (not (`KismetMathLibrary.NearlyEqual_FloatFloat` (`KismetMathLibrary.VSizeXY` (`Actor.GetVelocity` (`self.GetOwner`)))))
            (if (> (`self.WallHeight`) 100.0)
              (`KismetSystemLibrary.PrintString` "Front Flip")
              (`self.TryVault` "NewEnumerator2")
              (elif (> (`self.WallHeight`) 90.0)
                (`KismetSystemLibrary.PrintString` "Two Hand Vault")
                (`self.TryVault` "NewEnumerator1")
                (else
                  (`KismetSystemLibrary.PrintString` "One Hand Vault")
                  (`self.TryVault` "NewEnumerator0"))))
            (else
              (`KismetSystemLibrary.PrintString` "Mantle")))
          (else
            (`KismetSystemLibrary.PrintString` "Climb")))
        (else
          (`KismetSystemLibrary.PrintString` "Wall Height is over 300"))))))