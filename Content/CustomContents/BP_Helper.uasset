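; BP_Helper is a set of stateless math helper functions for offsetting positions and orienting toward surfaces.
; Six move functions shift a vector up or down along world Z, or forward, backward, left and right along a given rotation's axes.
; ReverseNormal builds a rotation from a surface normal's X axis and turns it 180 degrees, giving the rotation for the surface ahead of the player.
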(fn `MoveVectorBackward`
  (params (InVector :type "Vector Structure") (InRotation :type "Rotator Structure") (Subtract :type "Float (double-precision)"))
  (returns (ReturnValue :type "Vector Structure"))
  ;[1 1 1] ForwardVector의 반대 방향
  (return (- InVector (* (`KismetMathLibrary.GetForwardVector` InRotation) Subtract))))

(fn `MoveVectorDownward`
  (params (InVector :type "Vector Structure") (SubractValue :type "Float (double-precision)"))
  (returns (ReturnValue :type "Vector Structure"))
  ;[1 1 1] 현재 Vector 좌표를 Z축 밑으로 내려주는 함수
  (return (- InVector (`KismetMathLibrary.MakeVector` 0.0 0.0 SubractValue))))

(fn `MoveVectorForward`
  (params (InVector :type "Vector Structure") (InRotation :type "Rotator Structure") (AddValue :type "Float (double-precision)"))
  (returns (ReturnValue :type "Vector Structure"))
  ;[1 1 1] ForwardVector
  (return (+ InVector (* (`KismetMathLibrary.GetForwardVector` InRotation) AddValue))))

(fn `MoveVectorLeft`
  (params (InVector :type "Vector Structure") (InRotation :type "Rotator Structure") (MoveValue :type "Float (double-precision)"))
  (returns (ReturnValue :type "Vector Structure"))
  ;[1 1 1] Comment
  (return (- InVector (* (`KismetMathLibrary.GetRightVector` InRotation) MoveValue))))

(fn `MoveVectorRight`
  (params (InVector :type "Vector Structure") (InRotation :type "Rotator Structure") (MoveValue :type "Float (double-precision)"))
  (returns (ReturnValue :type "Vector Structure"))
  ;[1 1 1] Comment
  (return (+ InVector (* (`KismetMathLibrary.GetRightVector` InRotation) MoveValue))))

(fn `MoveVectorUpward`
  (params (InVector :type "Vector Structure") (AddValue :type "Float (double-precision)"))
  (returns (ReturnValue :type "Vector Structure"))
  ;[1 1 1] 현재 Vector에서 Z축으로 값을 더해주는 Vector 좌표를 Z축 위 방향으로 올려주는 함수
  (return (+ InVector (`KismetMathLibrary.MakeVector` 0.0 0.0 AddValue))))

(fn `ReverseNormal`
  (params (InNormal :type "Vector Structure"))
  (returns (ReturnValue :type "Rotator Structure"))
  ;[1 1 1] Player 전방 표면의 Rotation을 계산
  (return (`KismetMathLibrary.NormalizedDeltaRotator` (`KismetMathLibrary.MakeRotFromX` InNormal) (struct :`Yaw` 180.0))))