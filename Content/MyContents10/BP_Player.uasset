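; Player Blueprint that exercises trace queries with debug drawing and on-screen printing.
; Each tick, a capsule-radius sphere trace from the capsule's bottom prints the distance to whatever is below.
; IA_Fire line traces forward from BulletSpawnPoint and reports hits on "Wall"-tagged actors.
; Debug keys F and G cast rows of small sphere traces from scene points: F forward at stacked heights, G downward at forward steps.
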(event Input|EnhancedActionEvents|EnhancedInputActionIA_Fire
  (params (ActionValue :type Boolean) (ElapsedSeconds :type Float%20%28double-precision%29) (TriggeredSeconds :type Float%20%28double-precision%29) (InputAction :type Input%20Action%20Object%20Reference :default "/Game/MyContents10/Input/IA_Fire.IA_Fire"))
  (bind _bulletspawnpoint (Variables|Default|GetBulletSpawnPoint))
  (bind _returnvalue (Transformation|GetWorldLocation _bulletspawnpoint))
  ;[1 1 1] LineTrace
  (:Started
    (bind (_outhit _returnvalue_2) (Collision|LineTraceByChannel _returnvalue (+ _returnvalue (* (Math|Vector|GetForwardVector _bulletspawnpoint) 2e+04)) "TraceTypeQuery1" false 0 "ForDuration"))
    (if _returnvalue_2
      (if (Actor|ActorHasTag (.HitActor (Collision|BreakHitResult _outhit)) "Wall")
        (Development|PrintString "Hit Wall")))))

(event EventBeginPlay
  (|CallParentFunction) ; This node is disabled and will not be called.\nDrag off pins to build functionality.
)

(event Collision|EventActorBeginOverlap
  (params (OtherActor :type Actor%20Object%20Reference)))

(event EventTick
  (params (DeltaSeconds :type Float%20%28single-precision%29))
  ;[1 1 1] Player의 Distance값 받기
  (bind (_outhit _returnvalue) (Collision|SphereTraceByChannel (- (Transformation|GetActorLocation) (Math|Vector|MakeVector 0.0 0.0 (Variables|/Script/Engine.CapsuleComponent|GetCapsuleHalfHeight (Variables|Default|GetCapsuleComponent)))) (- (Transformation|GetActorLocation) "0.000000,0.000000,2000.000000") (Variables|/Script/Engine.CapsuleComponent|GetCapsuleRadius (Variables|Default|GetCapsuleComponent)) "TraceTypeQuery1" false 0 "ForOneFrame"))
  (if _returnvalue
    (Development|PrintString (Utilities|String|ToString(Float) (.Distance (Collision|BreakHitResult _outhit))))))

(event Input|KeyboardEvents|DebugKeyF
  (params (Key :type Key%20Structure :default "None") (ActionValue :type Input%20Action%20Value%20Structure))
  (:Pressed
    ;[1 1 1] Comment
    (for _index (range 0 3)
      (Collision|SphereTraceByChannel (+ (Transformation|GetWorldLocation (Variables|Default|GetCheckWallPoint)) (Math|Vector|MakeVector 0.0 0.0 (* _index 30))) (+ (+ (Transformation|GetWorldLocation (Variables|Default|GetCheckWallPoint)) (Math|Vector|MakeVector 0.0 0.0 (* _index 30))) (* (Math|Vector|GetForwardVector (Variables|Default|GetCheckWallPoint)) 1e+02)) 1e+01 "TraceTypeQuery1" false 0 "ForDuration"))))

(event Input|KeyboardEvents|DebugKeyG
  (params (Key :type Key%20Structure :default "None") (ActionValue :type Input%20Action%20Value%20Structure))
  (:Pressed
    ;[1 1 1] Comment
    (for _index (range 0 5)
      (Collision|SphereTraceByChannel (+ (Transformation|GetWorldLocation (Variables|Default|GetWallDistanceCheckPoint)) (* (Math|Vector|GetForwardVector (Variables|Default|GetWallDistanceCheckPoint)) (* _index 50))) (- (+ (Transformation|GetWorldLocation (Variables|Default|GetWallDistanceCheckPoint)) (* (Math|Vector|GetForwardVector (Variables|Default|GetWallDistanceCheckPoint)) (* _index 50))) "0.000000,0.000000,200.000000") 1e+01 "TraceTypeQuery1" false 0 "ForDuration"))))

(fn ConstructionScript
  (|CallParentFunction))