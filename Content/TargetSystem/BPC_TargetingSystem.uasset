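; Targeting component that finds enemies around its owning character and locks on to one in the camera's view.
; Initialize caches the character and gets its camera through a GetCameraMessage call.
; FindAllTargets sphere-traces pawns around the owner, accumulating unique "Enemy"-tagged actors in TargetEnemies.
; LockOnToTarget clears the lock, sweeps along camera forward, picks the known enemy nearest the owner, and fires OnLockOnNewTarget even if none qualifies.
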(fn `FindAllTargets`
  (returns (TargetEnemies :type "Array of Actor Object Reference"))
  (bind _returnvalue (`Actor.K2_GetActorLocation` (`self.GetOwner`)))
  (bind _outhits (`KismetSystemLibrary.SphereTraceMultiForObjects` _returnvalue _returnvalue (`self.TraceDistance`) (`|MakeArray` "ObjectTypeQuery3" :!type "EObjectTypeQuery Enum") false (`|MakeArray` (`self.GetOwner`)) "ForDuration"))
  (for _array_element _outhits
    (bind (_bblockinghit _binitialoverlap _time _distance _location _impactpoint _normal _impactnormal _physmat _hitactor) (`GameplayStatics.BreakHitResult` _array_element))
    (if (`Actor.ActorHasTag` _hitactor "Enemy")
      (`KismetArrayLibrary.Array_AddUnique` (`self.TargetEnemies`) _hitactor) ; 중복 x
    ))
  (return (`self.TargetEnemies`)))

(fn `Initialize`
  (bind _returnvalue (`self.GetOwner`))
  (bind _ascharacter (cast `Character` _returnvalue))
  (set `self.Character` _ascharacter)
  (bind _camera (message `/Game/TargetSystem/Interfaces/BPI_ThirdPersonCharacter.GetCamera` _returnvalue))
  (set `self.Camera` _camera))

(fn `LockOnToTarget`
  (returns (LockedOnTarget :type "Actor Object Reference"))
  (bind _camera (`self.Camera`))
  (bind _returnvalue (`SceneComponent.K2_GetComponentLocation` _camera))
  (set `self.LockedOnTarget` null) ; 디버깅을 위한 초기화
  (`/Engine/EditorBlueprintResources/StandardMacros.IsValid` (`self.LockedOnTarget`)
    (:`Is Not Valid`
      (set `self.ClosestDistance` (`self.TraceDistance`))
      (bind _outhits (`KismetSystemLibrary.SphereTraceMultiForObjects` :`Start` _returnvalue :`End` (+ _returnvalue (* (`SceneComponent.GetForwardVector` _camera) (`self.TraceDistance`))) :`Radius` (`self.RadiusToLockOn`) :`ObjectTypes` (`|MakeArray` "ObjectTypeQuery3" :!type "EObjectTypeQuery Enum") :`DrawDebugType` "ForDuration" :`TraceHitColor` (struct :`B` 1.0 :`A` 1.0)))
      (for _array_element _outhits
        (bind (_bblockinghit _binitialoverlap _time _distance _location _impactpoint _normal _impactnormal _physmat _hitactor) (`GameplayStatics.BreakHitResult` _array_element))
        ;[1 1 1] Comment
        (if (`KismetArrayLibrary.Array_Contains` (`self.TargetEnemies`) _hitactor)
          (bind _returnvalue_2 (`Actor.GetDistanceTo` _hitactor (`self.GetOwner`)))
          (if (< _returnvalue_2 (`self.ClosestDistance`))
            (set `self.ClosestDistance` _returnvalue_2)
            (set `self.LockedOnTarget` _hitactor) ; 가장 가까운 Actor를 LockedonTarget에 저장
          )))
      (`self.OnLockOnNewTarget`)
      (return (`self.LockedOnTarget`)))))