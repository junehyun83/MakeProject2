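; BP_HealthPotion is an item Blueprint for a health potion, inheriting its base item display behavior from a parent class.
; It overrides ShowItem, calling the parent version with the item name and count, then printing a formatted message built from its PotionType and EffectAmount variables.
; The event graph holds only disabled default events, and the file contains no logic that applies healing.
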(fn `ShowItem`
  (params (ItemName :type String) (ItemCount :type Integer))
  (`parent.ShowItem` ItemName ItemCount)
  (`KismetSystemLibrary.PrintString` (`KismetTextLibrary.Conv_TextToString` (`|FormatText` "{PotionType} will be added {EffectAmount}" (`self.PotionType`) (`self.EffectAmount`)))))

(fn `UserConstructionScript`
  (`parent.UserConstructionScript`))