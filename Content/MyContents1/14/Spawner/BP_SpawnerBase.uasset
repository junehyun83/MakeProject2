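; Base spawner Blueprint that repeatedly spawns actors of a configurable class, named as projectiles.
; A looping half-second timer starts on BeginPlay and spawns each actor at a random X within SpawnRange and at SpawnHeight on Z.
; StopTimer clears the stored timer handle to end spawning.
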(event `self.ReceiveBeginPlay`
  (bind _returnvalue (`KismetSystemLibrary.K2_SetTimerDelegate` (delegate `SpawnerProjectile`) 0.5 true))
  (set `self.TimeHandler` _returnvalue))

(event `SpawnerProjectile`
  (bind (_x _y) (`KismetMathLibrary.BreakVector2D` (`self.SpawnRange`)))
  (`|SpawnActorFromClass` (`self.SpawnClass`) (`KismetMathLibrary.MakeTransform` (`KismetMathLibrary.MakeVector` (`KismetMathLibrary.RandomFloatInRange` _x _y) 0.0 (`self.SpawnHeight`))) "Undefined" "MultiplyWithRoot" null null))

(event `StopTimer`
  (`KismetSystemLibrary.K2_ClearAndInvalidateTimerHandle` (`self.TimeHandler`)))

(fn `UserConstructionScript`)