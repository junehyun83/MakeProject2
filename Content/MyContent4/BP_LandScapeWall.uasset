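; Spline-driven landscape wall actor that builds a run of wall meshes along its spline in the construction script.
; When ActivateLineTrace is on, each spline point first snaps to the surface hit by a vertical line trace.
; Each segment fits a whole number of WallMesh copies from its bounding-box X width, stretching them evenly to fill the gap.
; Spline mesh components follow the curve, with tangents clamped to piece length.
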(fn `GetCurrentMeshCount`
  (returns (ReturnValue :type Boolean))
  (bind _output_get (set `self.CurrentMeshCount` (`KismetMathLibrary.FFloor` (`KismetMathLibrary.SafeDivide` (`self.CurrentSplineLength`) (`self.WallWidth`))))) ; 점과 점 사이에 몇개의 Mesh가 들어갈 수 있는지\n개수를 저장
  (return (> _output_get 0)))

(fn `GetCurrentSplineLength`
  (bind _returnvalue (`SplineComponent.GetDistanceAlongSplineAtSplinePoint` (`self.Spline`) (`self.CurrentPointIndex`)))
  (set `self.CurrentPointDistance` _returnvalue)
  (set `self.CurrentSplineLength` (- (`SplineComponent.GetDistanceAlongSplineAtSplinePoint` (`self.Spline`) (+ (`self.CurrentPointIndex`) 1)) _returnvalue)) ; Point와 Point 사이의 거리를 구함
)

(fn `GetWallWidth`
  (bind _wallmesh (`self.WallMesh`))
  (bind (_returnvalue_min _returnvalue_max) (break `Box` (`StaticMesh.GetBoundingBox` _wallmesh)))
  (bind _returnvalue_x (`KismetMathLibrary.BreakVector` (- _returnvalue_max _returnvalue_min)))
  (`/Engine/EditorBlueprintResources/StandardMacros.IsValid` _wallmesh
    (:`Is Valid`
      (set `self.WallWidth` _returnvalue_x))))

(fn `UserConstructionScript`
  (bind _spline (`self.Spline`))
  (bind _spline_2 (`self.Spline`))
  (`|ExecutionSequence`
    (:`then_0`
      (if (`self.ActivateLineTrace`)
        ;[1 1 1] Spline에 Point 정보
        (for _index (range (`SplineComponent.GetNumberOfSplinePoints` (`self.Spline`)))
          (bind (_returnvalue_x _returnvalue_y _returnvalue_z) (`KismetMathLibrary.BreakVector` (`SplineComponent.GetLocationAtSplinePoint` (`self.Spline`) _index "World")))
          (bind (_outhit _returnvalue) (`KismetSystemLibrary.LineTraceSingle` :`Start` (`KismetMathLibrary.MakeVector` _returnvalue_x _returnvalue_y (+ _returnvalue_z 10000.0)) :`End` (`KismetMathLibrary.MakeVector` _returnvalue_x _returnvalue_y (- _returnvalue_z 10000.0)) :`TraceChannel` "TraceTypeQuery1" :`DrawDebugType` "ForDuration")) ; z축 방향으로 위,아래를 LineTrace
          (if _returnvalue
            (`SplineComponent.SetLocationAtSplinePoint` (`self.Spline`) _index (`.Location` (`GameplayStatics.BreakHitResult` _outhit)) "World" true) ; 충돌이 발생한 곳으로\nSpline Point의 위치를 배치
          ))))
    (:`then_1`
      (`self.GetWallWidth`)
      (for _index_2 (range (+ (- (`SplineComponent.GetNumberOfSplinePoints` (`self.Spline`)) 2) 1))
        (set `self.CurrentPointIndex` _index_2)
        (`self.GetCurrentSplineLength`)
        (bind _returnvalue_2 (`self.GetCurrentMeshCount`))
        (if _returnvalue_2
          (set `self.CurrentModifiedMeshWidth` (/ (`self.CurrentSplineLength`) (`self.CurrentMeshCount`))) ; 점과 점 사이의 길이를 Mesh 개수로 나눠\n수정된 Mesh의 길이를 저장
          (for _index_3 (range (`self.CurrentMeshCount`))
            (bind _returnvalue_3 (`AddComponent|NODE_AddSplineMeshComponent-0`))
            (bind _returnvalue_4 (+ (* _index_3 (`self.CurrentModifiedMeshWidth`)) (`self.CurrentPointDistance`)))
            (bind _returnvalue_5 (+ (* (+ _index_3 1) (`self.CurrentModifiedMeshWidth`)) (`self.CurrentPointDistance`)))
            (`SplineMeshComponent.SetStartAndEnd` _returnvalue_3 (`SplineComponent.GetLocationAtDistanceAlongSpline` _spline_2 _returnvalue_4 "Local") (`KismetMathLibrary.ClampVectorSize` (`SplineComponent.GetTangentAtDistanceAlongSpline` _spline_2 _returnvalue_4 "Local") 0.0 (`self.CurrentModifiedMeshWidth`)) (`SplineComponent.GetLocationAtDistanceAlongSpline` _spline _returnvalue_5 "Local") (`KismetMathLibrary.ClampVectorSize` (`SplineComponent.GetTangentAtDistanceAlongSpline` _spline _returnvalue_5 "Local") 0.0 (`self.CurrentModifiedMeshWidth`)) true) ; SplineMeshComponent의\n시작점과 끝점을 정의
            (`StaticMeshComponent.SetStaticMesh` _returnvalue_3 (`self.WallMesh`))
            (`SceneComponent.K2_AttachToComponent` _returnvalue_3 (`self.Spline`) "None" "KeepRelative" "KeepRelative" "KeepRelative" true)))))))