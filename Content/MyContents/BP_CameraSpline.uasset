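; BP_CameraSpline is a spline actor meant to fly a level-placed camera along its path, though that logic is disconnected and BeginPlay does nothing.
; The unused chain finds the "SplineCamera"-tagged actor, makes it player 0's view target and plays a timeline scaled by CompleteTime.
; Timeline updates interpolate distance along the spline, setting the camera's world location and local-space roll and pitch, leaving yaw unwired.
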(event `self.ReceiveBeginPlay`)

(fn `UserConstructionScript`)